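; Game mode for a Nod vs GDI team match that spawns players at random team spawn points and decides round winners.
; It tracks living and dead players in team maps, plus living vehicle counts per team.
; When a player death leaves a team without players or vehicles, it flags the winner, then after a delay outputs stats, scores and announces the result.
; The timed respawn-all logic is disconnected.
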(event `AddToVehicleAliveMap`
  (params (isNodVehicle :type Boolean))
  ; Vehicle Account
  (if isNodVehicle
    (bind _result (`/Engine/EditorBlueprintResources/StandardMacros.IncrementInt` (`self.NodAliveVehicle`))
      (:`  `
        (set `self.NodAliveVehicle` _result)))
    (else
      (bind _result_2 (`/Engine/EditorBlueprintResources/StandardMacros.IncrementInt` (`self.GDIAliveVehicle`))
        (:`  `
          (set `self.GDIAliveVehicle` _result_2))))))

(event `self.K2_PostLogin`
  (params (NewPlayer :type "PlayerController Object Reference"))
  ; Spawn
  (`KismetArrayLibrary.Array_AddUnique` (`self.ConnectedPlayers`) NewPlayer)
  (bind _outactors (`GameplayStatics.GetAllActorsOfClass` "/Game/BP/SpawnPoint/BP_GDISpawnPoint.BP_GDISpawnPoint_C"))
  (set `self.GDISpawnPoint` _outactors)
  (bind _outactors_2 (`GameplayStatics.GetAllActorsOfClass` "/Game/BP/SpawnPoint/BP_NodSpawnPoint.BP_NodSpawnPoint_C"))
  (set `self.NodSpawnPoint` _outactors_2))

(event `RemoveToVehicleAliveMap`
  (params (isNodVehicle :type Boolean))
  ; Vehicle Account
  (if isNodVehicle
    (bind _result (`/Engine/EditorBlueprintResources/StandardMacros.DecrementInt` (`self.NodAliveVehicle`))
      (:`  `
        (set `self.NodAliveVehicle` _result)))
    (else
      (bind _result_2 (`/Engine/EditorBlueprintResources/StandardMacros.DecrementInt` (`self.GDIAliveVehicle`))
        (:`  `
          (set `self.GDIAliveVehicle` _result_2))))))

(event `RequestSpawnPlayer`
  (params (PlayerController :type "/Game/BP/PC_WorldRebalance Object Reference") (Team :type "Actor Class Reference"))
  (bind _returnvalue (== Team "/Game/BP/Player/BP_Nod.BP_Nod_C"))
  ; Spawn
  (`/Game/BP/PC_WorldRebalance.SpawnPlayer` PlayerController Team (select `bool` _returnvalue :`false` (`self.GetTransform` (`KismetArrayLibrary.Array_Random` (`self.GDISpawnPoint`))) :`true` (`self.GetTransform` (`KismetArrayLibrary.Array_Random` (`self.NodSpawnPoint`)))) _returnvalue))

(event `AddToPlayerAliveMap`
  (params (Player :type "/Game/BP/Player/BP_PlayerBase Object Reference (by ref)"))
  (bind _playerdead (`self.PlayerDead`))
  ; Track Player Live or Dead
  (if (`.ReturnValue` (`BlueprintMapLibrary.Map_Find` _playerdead Player))
    (`BlueprintMapLibrary.Map_Remove` _playerdead Player))
  (bind _playercontroller (message `/Game/BP/Player/Interface/BPI_PlayerController.GetPlayerControllerRef` (`Pawn.GetController` Player)))
  (`BlueprintMapLibrary.Map_Add` (`self.PlayerAlive`) Player (`/Game/BP/PC_WorldRebalance.Team` _playercontroller)))

(event `AddToPlayerDeadMap`
  (params (Player :type "/Game/BP/Player/BP_PlayerBase Object Reference"))
  (bind _playeralive (`self.PlayerAlive`))
  ; Track Player Live or Dead
  (if (`.ReturnValue` (`BlueprintMapLibrary.Map_Find` _playeralive Player))
    (`BlueprintMapLibrary.Map_Remove` _playeralive Player))
  (bind _playercontroller (message `/Game/BP/Player/Interface/BPI_PlayerController.GetPlayerControllerRef` (`Pawn.GetController` Player)))
  (`BlueprintMapLibrary.Map_Add` (`self.PlayerDead`) Player (`/Game/BP/PC_WorldRebalance.Team` _playercontroller))
  ; When One of a team member get to 0
  (bind (_nodalive _gdi_alive) (`self.m_CheckAmountOfLivingPlayer`))
  (bind _returnvalue (and (== _gdi_alive 0) (== (`self.GDIAliveVehicle`) 0)))
  (if (or (and (== _nodalive 0) (== (`self.NodAliveVehicle`) 0)) _returnvalue)
    (`|ExecutionSequence`
      (:`then_0`
        (set `self.isAccountingResult` true)
        (`KismetSystemLibrary.Delay` 5.0)
        (bind _asbp_game_state (cast `/Game/BP/BP_GameState` (`GameplayStatics.GetGameState`)))
        (bind _output_get (set `self.GameStats` _asbp_game_state))
        (`/Game/BP/BP_GameState.OutputData` _output_get)
        (`self.f_AddTeamScore`)
        (for _array_element (`self.PlayerSpawned`)
          (bind _returnvalue_2 (`Pawn.GetController` _array_element))
          (`/Engine/EditorBlueprintResources/StandardMacros.IsValid` _returnvalue_2
            (:`Is Valid`
              ; FPS Player Controller
              (bind _playercontroller_2 (message `/Game/BP/Player/Interface/BPI_PlayerController.GetPlayerControllerRef` _returnvalue_2))
              (bind _values (`BlueprintMapLibrary.Map_Values` (`self.PlayerAlive`)))
              (bind _output (`|GetArrayItem` _values))
              (`/Game/BP/PC_WorldRebalance.UpdateTeamWinAnnouncement` _playercontroller_2 _output (`KismetMathLibrary.SelectInt` (`self.NodScore`) (`self.GDI Score`) (== _output "/Game/BP/Player/BP_Nod.BP_Nod_C")) (`self.RespawnTimer`)))))
        ; Clear Live Dead Data
        (`BlueprintMapLibrary.Map_Clear` (`self.PlayerAlive`))
        (`BlueprintMapLibrary.Map_Clear` (`self.PlayerDead`))
        (set `self.isAccountingResult` false))
      (:`then_1`
        ; get isNodWin
        (if _returnvalue
          (set `self.isNodWin` true)
          (`KismetSystemLibrary.PrintString` "Nod win" true true (struct :`R` 1.0 :`G` 0.068094 :`A` 1.0) 100.0)
          (else
            (set `self.isNodWin` false)
            (`KismetSystemLibrary.PrintString` "GDI win" true true (struct :`R` 1.0 :`G` 0.924858 :`A` 1.0) 100.0)))))))

(event `AddToPlayerSpawnedArray`
  (params (Player :type "/Game/BP/Player/BP_PlayerBase Object Reference"))
  (bind _playerspawned (`self.PlayerSpawned`))
  ; Get Player Num
  (`KismetArrayLibrary.Array_Set` _playerspawned (`KismetArrayLibrary.Array_Length` _playerspawned) Player true))

(fn `f_AddTeamScore`
  (if (and (== (`self.GDIAlive`) 0) (== (`self.GDIAliveVehicle`) 0))
    (`/Engine/EditorBlueprintResources/StandardMacros.IncrementInt` (`self.NodScore`))
    (else
      (`/Engine/EditorBlueprintResources/StandardMacros.IncrementInt` (`self.GDI Score`)))))

(fn `GetGameModeRef`
  (returns (GameMode :type "/Game/BP/GM_WorldRebalance Object Reference"))
  (return self))

(fn `GetPlayerStateRef`
  (returns (PlayerState :type "/Game/BP/BP_PlayerState Object Reference"))
  (return null))

(fn `UserConstructionScript`)