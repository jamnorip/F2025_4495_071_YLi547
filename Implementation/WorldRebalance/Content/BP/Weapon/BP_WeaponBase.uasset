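; Base weapon actor that spawns as a physics object and offers itself for pickup to overlapping players.
; On BeginPlay it initializes magazine and reserve ammo from weapon info looked up by name.
; Server-only sphere overlap polls until the weapon is interactable, then adds it to a player's overlapped weapons unless their inventory holds that type.
; It skips the player who just dropped it, resetting that player's dropped-weapon reference on end overlap.
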(event `SRV_InitializeWeapon`
  (bind (_weaponinfo_name _weaponinfo_type _weaponinfo_thumbnail _weaponinfo_class _weaponinfo_maxammoinmag _weaponinfo_maxextraammo) (break `/Game/BP/Struct/ST_WeaponInfo` (`/Game/BP/Library/BP_FunctionLibrary.f_GetWeaponInfo` (`self.WeaponName`))))
  ; Read Ammo Account
  (set `self.CurrentAmmoInMag` _weaponinfo_maxammoinmag)
  (set `self.CurrentExtraAmmo` _weaponinfo_maxextraammo))

(event `self.ReceiveBeginPlay`
  ;[0 0 0 0.5] Begin Play
  (`PrimitiveComponent.SetSimulatePhysics` (`self.Weapon`) true)
  ; Read Ammo Account
  (`self.SRV_InitializeWeapon`))

(event `self.CollisionSphere.OnComponentBeginOverlap`
  (params (OverlappedComponent :type "PrimitiveComponent Object Reference") (OtherActor :type "Actor Object Reference") (OtherComp :type "PrimitiveComponent Object Reference") (OtherBodyIndex :type Integer) (bFromSweep :type Boolean) (SweepResult :type "HitResult Structure (by ref)"))
  (bind _overlappingactors (`self.GetOverlappingActors` "/Game/BP/Player/BP_PlayerBase.BP_PlayerBase_C"))
  (bind (_weaponinfo_name _weaponinfo_type) (break `/Game/BP/Struct/ST_WeaponInfo` (`/Game/BP/Library/BP_FunctionLibrary.f_GetWeaponInfo` (`self.WeaponName`))))
  (if (`self.ActorHasTag` OtherActor "Player")
    (`/Engine/EditorBlueprintResources/ActorMacros.Switch Has Authority` ; only run in the server
      (:`Authority`
        (if (`self.bCanBeInteractiveWith`) :!label _label
          ; Cal how many players are here
          (if (`KismetArrayLibrary.Array_IsNotEmpty` _overlappingactors)
            (if (> (`KismetArrayLibrary.Array_Length` _overlappingactors) 1)
              (for _array_element _overlappingactors
                (bind _player (message `/Game/BP/Player/Interface/BPI_PlayerBase.GetPlayerRef` _array_element))
                (if (!= (`/Game/BP/Player/BP_PlayerBase.Dropped Weapon` _player) self)
                  (set `self.InteractingPlayer` _player)
                  (break)))
              ; Inventary
              (for _array_element_2 (`/Game/BP/Player/BP_PlayerBase.WeaponInventory` (`self.InteractingPlayer`)) :!label _label_2
                (bind (_weaponinfo_name_2 _weaponinfo_type_2) (break `/Game/BP/Struct/ST_WeaponInfo` (`/Game/BP/Library/BP_FunctionLibrary.f_GetWeaponInfo` (`/Game/BP/Weapon/BP_WeaponBase.WeaponName` _array_element_2))))
                (if (`|EnumEquality` _weaponinfo_type_2 _weaponinfo_type)
                  (set `/Game/BP/Player/BP_PlayerBase.bCanLootWeapon` false (`self.InteractingPlayer`))
                  (break)))
              (if (`/Game/BP/Player/BP_PlayerBase.bCanLootWeapon` (`self.InteractingPlayer`))
                (`/Game/BP/Player/BP_PlayerBase.AddOverlappedWeapon` (`self.InteractingPlayer`) self)
                (else
                  (set `/Game/BP/Player/BP_PlayerBase.bCanLootWeapon` true (`self.InteractingPlayer`)) ; set as default for the future
                ))
              (else
                (bind _player_2 (message `/Game/BP/Player/Interface/BPI_PlayerBase.GetPlayerRef` (`|GetArrayItem` _overlappingactors)))
                (bind _output_get (set `self.InteractingPlayer` _player_2))
                (if (!= (`/Game/BP/Player/BP_PlayerBase.Dropped Weapon` _output_get) self)
                  (goto _label_2)))))
          (else
            (`KismetSystemLibrary.Delay` 0.01)
            (goto _label)))))))

(event `self.CollisionSphere.OnComponentEndOverlap`
  (params (OverlappedComponent :type "PrimitiveComponent Object Reference") (OtherActor :type "Actor Object Reference") (OtherComp :type "PrimitiveComponent Object Reference") (OtherBodyIndex :type Integer))
  ; Reset the dropped weapon to none if player out of the rigger
  (if (`self.ActorHasTag` OtherActor "Player")
    (`/Engine/EditorBlueprintResources/ActorMacros.Switch Has Authority`
      (:`Authority`
        (bind _player (message `/Game/BP/Player/Interface/BPI_PlayerBase.GetPlayerRef` OtherActor))
        (`/Game/BP/Player/BP_PlayerBase.SetDroppedWeapon` _player null)))))

(fn `GetWeaponRef`
  (returns (Weapon :type "/Game/BP/Weapon/BP_WeaponBase Object Reference"))
  (return self))

(fn `UserConstructionScript`)