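; Player controller for a team-based match (GDI vs Nod) that handles team selection, pawn spawning and possession, and the player's HUD.
; Team choices go through a server event to the GameMode, while SpawnPlayer spawns and possesses the team's pawn, then switches the client to game input.
; Client events show or hide lazily created, cached widgets, swap to a tank crosshair for vehicles, and update team scores with win/lose sounds.
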(event `self.ReceiveBeginPlay`
  (`self.ShowHideWidget` "NewEnumerator0" true)
  (bind _gamemode (message `/Game/BP/Player/Interface/BPI_GameMode.GetGameModeRef` (`GameplayStatics.GetGameMode`)))
  (set `self.Game Mode` _gamemode)
  (bind _returnvalue (`GameplayStatics.GetActorOfClass` "/Script/Engine.CameraActor")) ; Select the camera for bg menu
  (`self.SetViewTargetWithBlend` _returnvalue)
  (`WidgetBlueprintLibrary.SetInputMode_UIOnlyEx` self null))

(event `ShowHideWidget`
  (params (Widget :type "/Game/BP/Enum/E_GameWidget Enum" :default "NewEnumerator0") (Show :type Boolean))
  (`self.Client_ShowHideWidget` Widget Show))

(event `Client_ShowHideWidget`
  (params (Widget :type "/Game/BP/Enum/E_GameWidget Enum" :default "NewEnumerator0") (Show :type Boolean))
  (if Show
    (`self.f_ShowWidget` Widget)
    (else
      (`self.f_HideWidget` Widget))))

(event `SelectTeam`
  (params (Team :type "Actor Class Reference") (PlayerName :type String))
  (`self.SRV_SelectTeam` Team PlayerName))

(event `SRV_SelectTeam`
  (params (Team :type "Actor Class Reference") (PlayerName :type String))
  (bind _output_get (set `self.Team` Team))
  (`/Game/BP/GM_WorldRebalance.RequestSpawnPlayer` (`self.Game Mode`) self _output_get)
  ;[1 1 0 0.5] for Output playerName
  (set `self.PlayerName` PlayerName))

(event `CL_LoadVehicleWidget`
  ;[0.15 0 0 0.5] VehicleWidget
  (`self.ShowHideWidget` "NewEnumerator3") ; Team
  (`self.ShowHideWidget` "NewEnumerator4") ; Team
  (`self.ShowHideWidget` "NewEnumerator6" true) ; Team
)

(event `SpawnPlayer`
  (params (Team :type "Actor Class Reference") (SpawnTransform :type "Transform Structure") (isNod :type Boolean))
  (set `self.isNod` isNod)
  (bind _returnvalue (`|SpawnActorFromClass` Team SpawnTransform "AdjustIfPossibleButAlwaysSpawn" "MultiplyWithRoot" null null))
  (bind _output_get (set `self.PlayerPawn` _returnvalue))
  (bind _player (message `/Game/BP/Player/Interface/BPI_PlayerBase.GetPlayerRef` _output_get))
  (`self.Possess` _player)
  (`self.Client_SpawnPlayer`)
  ;[1 1 0 0.5] Comment
  (set `self.JoinTime` (`KismetMathLibrary.Now`)))

(event `CL_RemoveVehicleWidget`
  ;[0.15 0 0 0.5] VehicleWidget
  (`self.ShowHideWidget` "NewEnumerator6") ; Team
  (`self.ShowHideWidget` "NewEnumerator4" true) ; Team
  (`self.ShowHideWidget` "NewEnumerator3" true) ; Team
)

(event `Client_SpawnPlayer`
  (`self.ShowHideWidget` "NewEnumerator0") ; Team
  (`self.ShowHideWidget` "NewEnumerator3" true) ; Playing
  (`self.ShowHideWidget` "NewEnumerator4" true) ; Crosshair
  (`WidgetBlueprintLibrary.SetInputMode_GameOnly` self)
  (set `self.bShowMouseCursor` false))

(event `UpdateTeamWinAnnouncement`
  (params (WinTeam :type "Actor Class Reference") (Score :type Integer) (DisplayTime :type "Float (double-precision)"))
  (`self.CL_UpdateTeamWinAnnouncement` WinTeam Score DisplayTime))

(event `CL_UpdateTeamWinAnnouncement`
  (params (WinTeam :type "Actor Class Reference") (Score :type Integer) (DisplayTime :type "Float (double-precision)"))
  (bind _wb_mainplaying (`self.WB_MainPlaying`))
  (`/Game/UI/WB_MainPlaying.UpdateTeamWinAnnouncementUI` (`self.WB_MainPlaying`) WinTeam DisplayTime)
  (if (== WinTeam "/Game/BP/Player/BP_Nod.BP_Nod_C")
    (`/Game/UI/WB_MainPlaying.UpdateNodScoreUI` _wb_mainplaying Score)
    (else
      (`/Game/UI/WB_MainPlaying.UpdateGDIScoreUI` _wb_mainplaying Score)))
  ; Play win or lose sound
  (`GameplayStatics.PlaySound2D` (select `bool` (== WinTeam (`self.Team`)) :`false` "/Game/FX/Sound/GrenadeLauncher/Cues/GrenadeLauncherA_Fire_Cue.GrenadeLauncherA_Fire_Cue" :`true` "/Game/FX/Sound/Rifle/Cues/Rifle_ReloadInsert_Cue.Rifle_ReloadInsert_Cue" :!type "SoundBase Object Reference") 1.0 1.0 0.0 null null))

(fn `f_HideWidget`
  (params (Widget :type "/Game/BP/Enum/E_GameWidget Enum" :default "NewEnumerator0"))
  (switch `/Game/BP/Enum/E_GameWidget` Widget
    (:`NewEnumerator3`
      (bind _wb_mainplaying (`self.WB_MainPlaying`)
        (:`then`
          (`Widget.RemoveFromParent` _wb_mainplaying))
        (:`else`)))
    (:`NewEnumerator0`
      (bind _wb_teamselection (`self.WB_TeamSelection`)
        (:`then`
          (`Widget.RemoveFromParent` _wb_teamselection))
        (:`else`)))
    (:`NewEnumerator4`
      (bind _wb_crosshair (`self.WB_Crosshair`)
        (:`then`
          (`Widget.RemoveFromParent` _wb_crosshair))
        (:`else`)))
    (:`NewEnumerator6`
      (bind _wb_tankcrosshair (`self.WB_TankCrosshair`)
        (:`then`
          (`Widget.RemoveFromParent` _wb_tankcrosshair))
        (:`else`)))))

(fn `f_ShowWidget`
  (params (Widget :type "/Game/BP/Enum/E_GameWidget Enum" :default "NewEnumerator0"))
  (switch `/Game/BP/Enum/E_GameWidget` Widget
    (:`NewEnumerator3`
      (`self.WB_MainPlaying`
        (:`then`
          _)
        (:`else`
          (bind _returnvalue (`|CreateWidget` "/Game/UI/WB_MainPlaying.WB_MainPlaying_C"))
          (bind _output_get (set `self.WB_MainPlaying` _returnvalue))))
      (`UserWidget.AddToViewport` _output_get 0))
    (:`NewEnumerator0`
      (`self.WB_TeamSelection` ; Not Valid is not created
        (:`then`
          _)
        (:`else`
          (bind _returnvalue_2 (`|CreateWidget` "/Game/UI/WB_TeamSelection.WB_TeamSelection_C"))
          (bind _output_get_2 (set `self.WB_TeamSelection` _returnvalue_2))))
      (`UserWidget.AddToViewport` _output_get_2 0))
    (:`NewEnumerator4`
      (`self.WB_Crosshair`
        (:`then`
          _)
        (:`else`
          (bind _returnvalue_3 (`|CreateWidget` "/Game/UI/WB_Crosshair.WB_Crosshair_C"))
          (bind _output_get_3 (set `self.WB_Crosshair` _returnvalue_3))))
      (`UserWidget.AddToViewport` _output_get_3 0))
    (:`NewEnumerator6`
      (`self.WB_TankCrosshair`
        (:`then`
          _)
        (:`else`
          (bind _returnvalue_4 (`|CreateWidget` "/Game/UI/WB_TankCrosshair.WB_TankCrosshair_C" null null))
          (bind _output_get_4 (set `self.WB_TankCrosshair` _returnvalue_4))))
      (`UserWidget.AddToViewport` _output_get_4 0))))

(fn `GetPlayerControllerRef`
  (returns (PlayerController :type "/Game/BP/PC_WorldRebalance Object Reference"))
  (return self))

(fn `UserConstructionScript`)