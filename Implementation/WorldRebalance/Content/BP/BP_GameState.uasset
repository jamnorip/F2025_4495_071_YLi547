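; BP_GameState is a game state Blueprint that exports per-player match statistics to a text file.
; Its OutputData event gathers all BP_PlayerBase actors and reads each one's PlayerController for identity, vehicle, session timing, combat totals and win status.
; Each player becomes a comma-separated line appended to a Text array, which SaveArrayText writes to PlayerOutput.txt in the project directory, overwriting any existing file.
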(event `self.ReceiveBeginPlay`)

(event `OutputData`
  (bind _outactors (`GameplayStatics.GetAllActorsOfClass` "/Game/BP/Player/BP_PlayerBase.BP_PlayerBase_C"))
  (bind _output_get (set `self.Players` _outactors))
  (for _array_element _output_get
    (bind _playercontroller (`/Game/BP/Player/BP_PlayerBase.PlayerController` _array_element))
    (`KismetArrayLibrary.Array_Add` (`self.Text`) (`KismetStringLibrary.Concat_StrStr` (`/Game/BP/PC_WorldRebalance.PlayerName` _playercontroller) ", " (`/Game/BP/PC_WorldRebalance.Vehicle` _playercontroller) ", " (`KismetTextLibrary.Conv_TextToString` (`KismetTextLibrary.AsDateTime_DateTime` (`/Game/BP/PC_WorldRebalance.JoinTime` _playercontroller))) ", " (`KismetTextLibrary.Conv_TextToString` (`KismetTextLibrary.AsDateTime_DateTime` (`/Game/BP/PC_WorldRebalance.LeaveTime` _playercontroller))) ", " (`/Game/BP/PC_WorldRebalance.PlayDuration` _playercontroller) ", " (`KismetStringLibrary.Conv_IntToString` (`PC_Trooper.GetKillCount` _playercontroller)) ", " (`KismetStringLibrary.Conv_IntToString` (`/Game/BP/PC_WorldRebalance.DeathCount` _playercontroller)) ", " (`KismetStringLibrary.Conv_BoolToString` (`/Game/BP/PC_WorldRebalance.IsWin` _playercontroller)) ", " (`KismetStringLibrary.Conv_IntToString` (`PC_Trooper.GetDamageDealt` _playercontroller)) ", " (`KismetStringLibrary.Conv_IntToString` (`/Game/BP/PC_WorldRebalance.DamageGet` _playercontroller)))))
  (`TextFileManager.SaveArrayText` (`KismetSystemLibrary.GetProjectDirectory`) "PlayerOutput.txt" (`self.Text`) true))

(fn `UserConstructionScript`)