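; Base drivable tank that players board via an overlap volume, drive, fire and exit with F, which hands possession back to their character.
; Enhanced Input relays throttle, firing and gimbal/spring-arm aim through SRV events to TankMovement and the tracks, with right input feeding the left track and vice versa.
; Tick polls hit and death flags to update health UI or eject the driver, deregister from the GameMode and destroy the tank.
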(event `self.ReceiveBeginPlay`
  ; Load Mapping
  (`|ExecutionSequence`
    (:`then_0`
      ;; Movement
      (bind _aspc_tank (cast `/Game/Tank/PC_Tank` (`self.GetController`)))
      (`EnhancedInputSubsystemInterface.AddMappingContext` (pcsubsystem `EnhancedInputLocalPlayerSubsystem` _aspc_tank) "/Game/Tank/Input/MC_Tank.MC_Tank" 0 (struct)))
    (:`then_1`
      (`TankMovementComponent.Initialise` (`self.TankMovement`) (`self.TankTrack_BL`) (`self.TankTrack_BR`) :!label _label))
    (:`then_2`
      (`self.Initialise` (`self.BarrelComp`) (`self.TurretComp`)))
    (:`then_3`
      (`self.SetCurrentHealth` (`KismetMathLibrary.Conv_IntToDouble` (`self.StartingHealth`))))))

(event `SRV_InitialiseComponent`
  ; Load Mapping
  (goto _label))

(event `SRV_RemoveVehicle`
  (params (isNodVehicle :type Boolean))
  (bind _character (`self.Character`))
  ; Connect to Gamemode
  (`/Engine/EditorBlueprintResources/StandardMacros.IsValid` _character
    (:`Is Valid`
      (`/Game/BP/GM_WorldRebalance.RemoveToVehicleAliveMap` (`/Game/BP/Player/BP_PlayerBase.GameMode` _character) isNodVehicle))))

(event `M_AimTowardCrosshair`
  (`self.SVR_AimTowardCrosshair`))

(event `SVR_AimTowardCrosshair`
  (`self.AimTowardCrosshair`))

(event `self.ReceiveTick`
  (params (DeltaSeconds :type "Float (single-precision)"))
  (bind _character (`self.Character`))
  (`|ExecutionSequence`
    (:`then_0`
      ; Death
      (if (`self.IsDead`)
        (`/Engine/EditorBlueprintResources/StandardMacros.IsValid` (`self.Character`)
          (:`Is Valid`
            (`self.SRV_RemoveVehicle` (`self.isNodVehicle`))
            (`self.RPC_SRV_UnPossessVehicle`))
          (:`Is Not Valid`
            _))
        (`KismetSystemLibrary.Delay` 0.5)
        ;;[1 0 0 0.5] D
        (`self.K2_DestroyActor`)))
    (:`then_1`
      ;[1 1 0 0.5] DamageGet
      (if (`self.isOnHit`)
        (`/Engine/EditorBlueprintResources/StandardMacros.IsValid` _character
          (:`Is Valid`
            (set `/Game/BP/PC_WorldRebalance.DamageGet` (`KismetMathLibrary.FTrunc` (`self.GetDamaged`)) (`/Game/BP/Player/BP_PlayerBase.PlayerController` _character))
            (`self.SetOnHit`)
            (`self.CL_FireHealthWidget`)))))))

(event `CL_FireHealthWidget`
  (bind _playercontroller (message `/Game/BP/Player/Interface/BPI_PlayerController.GetPlayerControllerRef` (`self.GetLocalViewingPlayerController`)))
  (`/Game/UI/WB_TankCrosshair.UpdateHealthbar` (`/Game/BP/PC_WorldRebalance.WB_TankCrosshair` _playercontroller) (`self.GetHealthPercent`)))

(event `Key|F`
  (params (Key :type "Key Structure"))
  ; Drive
  (:`Pressed`
    (`self.SRV_OutofVehicle`)))

(event `SRV_OutofVehicle`
  ; Drive
  (`self.SRV_RemoveVehicle` (`self.isNodVehicle`))
  (`self.RPC_SRV_UnPossessVehicle`))

(event `RPC_SRV_UnpossessVehicle`
  ; Drive
  (`self.M_RPC_UnpossessVehicle`))

(event `M_RPC_UnpossessVehicle`
  (bind _character (`self.Character`))
  (bind _character_2 (`self.Character`))
  ; Drive
  (set `self.isFullofDriver` false)
  (`/Engine/EditorBlueprintResources/StandardMacros.IsValid` _character_2
    (:`Is Valid`
      (set `/Game/BP/Player/BP_PlayerBase.IsDriving` false _character_2)
      (set `self.isFullofDriver` false)
      (`/Engine/EditorBlueprintResources/StandardMacros.IsValid` _character_2
        (:`Is Valid`
          (bind _aspc_world_rebalance (cast `/Game/BP/PC_WorldRebalance` (`self.GetController`)))
          (`Controller.UnPossess` _aspc_world_rebalance)
          (set `self.PC_intank` null)
          (`/Engine/EditorBlueprintResources/StandardMacros.IsValid` _character
            (:`Is Valid`
              ;; Remove Vehicle Widget
              (`/Game/BP/PC_WorldRebalance.CL_RemoveVehicleWidget` (`/Game/BP/Player/BP_PlayerBase.PlayerController` _character))
              (`Controller.Possess` _aspc_world_rebalance _character)
              (`/Game/BP/Player/BP_PlayerBase.RPC_SRV_PossessCharacter` _character))))))))

(event `CL_UIRoundAmmo`
  ; Fire
  (bind _playercontroller (message `/Game/BP/Player/Interface/BPI_PlayerController.GetPlayerControllerRef` (`self.GetLocalViewingPlayerController`)))
  (`/Game/UI/WB_TankCrosshair.UpdateRounds` (`/Game/BP/PC_WorldRebalance.WB_TankCrosshair` _playercontroller) (`self.GetRoundsLeft`)))

(event `SRV_Fire`
  ; Fire
  (`self.Fire`))

(event `EnhancedInput|/Game/Tank/Input/IA_Fire`
  (params (ActionValue :type Boolean) (ElapsedSeconds :type "Float (double-precision)") (TriggeredSeconds :type "Float (double-precision)") (InputAction :type "InputAction Object Reference" :default "/Game/Tank/Input/IA_Fire.IA_Fire"))
  ; Fire
  (:`Triggered`
    (`self.CL_UIRoundAmmo`)
    (`self.SRV_Fire`)))

(event `EnhancedInput|/Game/Tank/Input/IA_RightTrackThrottle`
  (params (ActionValue :type "Float (double-precision)") (ElapsedSeconds :type "Float (double-precision)") (TriggeredSeconds :type "Float (double-precision)") (InputAction :type "InputAction Object Reference" :default "/Game/Tank/Input/IA_RightTrackThrottle.IA_RightTrackThrottle"))
  ; Movement
  (:`Triggered`
    (`self.SRV_RightTrackThrottle` ActionValue)))

(event `SRV_RightTrackThrottle`
  (params (`Action Value` :type "Float (double-precision)"))
  ; Movement
  (`TankTrack.SetThrottle` (`self.TankTrack_BL`) (* `Action Value` (`self.TurningWheelRotationValue`))))

(event `C_SwapCam`
  ; Swap Cam Third Person View - First Person View
  (`ActorComponent.ToggleActive` (`self.FirstPersonCam`))
  (`ActorComponent.ToggleActive` (`self.ThridPersonCam`)))

(event `EnhancedInput|/Game/Tank/Input/IA_SwapCam`
  (params (ActionValue :type Boolean) (ElapsedSeconds :type "Float (double-precision)") (TriggeredSeconds :type "Float (double-precision)") (InputAction :type "InputAction Object Reference" :default "/Game/Tank/Input/IA_SwapCam.IA_SwapCam"))
  ; Swap Cam Third Person View - First Person View
  (:`Triggered`
    (`self.C_SwapCam`)))

(event `EnhancedInput|/Game/Tank/Input/IA_AimAzimuth`
  (params (ActionValue :type "Vector2D Structure") (ElapsedSeconds :type "Float (double-precision)") (TriggeredSeconds :type "Float (double-precision)") (InputAction :type "InputAction Object Reference" :default "/Game/Tank/Input/IA_AimAzimuth.IA_AimAzimuth"))
  ; Camera
  (:`Triggered`
    (`self.M_AimZimuth` ActionValue_X ActionValue_Y)))

(event `EnhancedInput|/Game/Tank/Input/IA_LeftTrackThrottle`
  (params (ActionValue :type "Float (double-precision)") (ElapsedSeconds :type "Float (double-precision)") (TriggeredSeconds :type "Float (double-precision)") (InputAction :type "InputAction Object Reference" :default "/Game/Tank/Input/IA_LeftTrackThrottle.IA_LeftTrackThrottle"))
  ; Movement
  (:`Triggered`
    (`self.SRV_LeftTrackThrottle` ActionValue)))

(event `SRV_LeftTrackThrottle`
  (params (`Action Value` :type "Float (double-precision)"))
  ; Movement
  (`TankTrack.SetThrottle` (`self.TankTrack_BR`) (* `Action Value` (`self.TurningWheelRotationValue`))))

(event `SRV_AimZimuth`
  (params (`Action Value X` :type "Float (double-precision)") (`Action Value Y` :type "Float (double-precision)"))
  ; Camera
  (`|ExecutionSequence`
    (:`then_0`
      (`SceneComponent.K2_AddLocalRotation` (`self.AzimuthGimbalScene`) (`KismetMathLibrary.MakeRotator` 0.0 0.0 (* `Action Value X` -1.0)) false false))
    (:`then_1`
      (`SceneComponent.K2_AddLocalRotation` (`self.SpringArm`) (`KismetMathLibrary.MakeRotator` 0.0 (* `Action Value Y` -1.0)) false false))))

(event `EnhancedInput|/Game/Tank/Input/IA_TrackBack`
  (params (ActionValue :type "Float (double-precision)") (ElapsedSeconds :type "Float (double-precision)") (TriggeredSeconds :type "Float (double-precision)") (InputAction :type "InputAction Object Reference" :default "/Game/Tank/Input/IA_TrackBack.IA_TrackBack"))
  ; Movement
  (:`Triggered`
    (`self.SRV_TrackBack` ActionValue)))

(event `SRV_TrackBack`
  (params (`Action Value` :type "Float (double-precision)"))
  ; Movement
  (`TankMovementComponent.IntendMoveForward` (`self.TankMovement`) (* `Action Value` (`self.TurningWheelBackValue`))))

(event `M_AimZimuth`
  (params (`Action Value X` :type "Float (double-precision)") (`Action Value Y` :type "Float (double-precision)"))
  ; Camera
  (`self.SRV_AimZimuth` `Action Value X` `Action Value Y`))

(event `EnhancedInput|/Game/Tank/Input/IA_TrackForward`
  (params (ActionValue :type "Float (double-precision)") (ElapsedSeconds :type "Float (double-precision)") (TriggeredSeconds :type "Float (double-precision)") (InputAction :type "InputAction Object Reference" :default "/Game/Tank/Input/IA_TrackForward.IA_TrackForward"))
  ; Movement
  (:`Triggered`
    (`self.SRV_TrackForward` ActionValue)))

(event `SRV_TrackForward`
  (params (`Action Value` :type "Float (double-precision)"))
  ; Movement
  (`TankMovementComponent.IntendMoveForward` (`self.TankMovement`) (* `Action Value` (`self.TurningWheelForwardValue`))))

(event `self.DriveCollision.OnComponentBeginOverlap`
  (params (OverlappedComponent :type "PrimitiveComponent Object Reference") (OtherActor :type "Actor Object Reference") (OtherComp :type "PrimitiveComponent Object Reference") (OtherBodyIndex :type Integer) (bFromSweep :type Boolean) (SweepResult :type "HitResult Structure (by ref)"))
  (bind _asbp_player_base (cast `/Game/BP/Player/BP_PlayerBase` OtherActor))
  (set `/Game/BP/Player/BP_PlayerBase.Vehicle` self _asbp_player_base)
  (set `/Game/BP/Player/BP_PlayerBase.OverlapVehicle` true _asbp_player_base))

(event `self.DriveCollision.OnComponentEndOverlap`
  (params (OverlappedComponent :type "PrimitiveComponent Object Reference") (OtherActor :type "Actor Object Reference") (OtherComp :type "PrimitiveComponent Object Reference") (OtherBodyIndex :type Integer))
  (bind _asbp_player_base (cast `/Game/BP/Player/BP_PlayerBase` OtherActor))
  (set `/Game/BP/Player/BP_PlayerBase.OverlapVehicle` false _asbp_player_base))

(fn `UserConstructionScript`)